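; Game mode for the creature race: spawns a track generator on BeginPlay, then sets up cursor input, a fade widget and music.
; StartRace spawns behavior-tree-driven Chao at random track spawn points, held by a wait-for-signal gameplay effect that is removed after a short delay.
; Finishers receive a finish-line gameplay effect, and getters expose the active track and its spline.
; EndRace is an empty stub.
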(event Custom|StartRace
  (Utilities|Array|Clear (Variables|Default|GetFinishedCreatureActorArray))
  (CallFunction|SpawnCreatures)
  (Utilities|FlowControl|Delay 1.0)
  (for _array_element (Variables|Default|GetSpawnedCreatures)
    (GameplayEffects|RemoveActiveGameplayEffectbySourceEffect (Ability|GetAbilitySystemComponent _array_element) "/Game/CreatureOasis/Core/Characters/Chao/GameplayEffects/Racing/GE_WaitForStartSignal_BP.GE_WaitForStartSignal_BP_C" 0 -1)))

(event Custom|EndRace)

(event EventProcessFinishedCreature
  (params (FinishedCreatureActor :type Actor%20Object%20Reference))
  (bind _returnvalue (Ability|GetAbilitySystemComponent FinishedCreatureActor))
  (Utilities|IsValid _returnvalue
    (:Is%20Valid
      (GameplayEffects|ApplyGameplayEffectToSelf :self _returnvalue :GameplayEffectClass "/Game/CreatureOasis/Core/Characters/Chao/GameplayEffects/Racing/GE_ReachedFinishLine_BP.GE_ReachedFinishLine_BP_C"))))

(event EventBeginPlay
  (bind _returnvalue (Game|GetPlayerController 0))
  (Utilities|FlowControl|Sequence
    (:then_0
      (bind _returnvalue_2 (Game|SpawnActorfromClass "/Script/CreatureOasis.TrackGeneratorActor" (Variables|Default|GetTrackGeneratorSpawnTransform) "AlwaysSpawn" 0 0))
      (Variables|Default|SetActiveTrackGenerator _returnvalue_2))
    (:then_1
      (Input|SetInputModeGameandUI _returnvalue 0 "DoNotLock" false)
      (Variables|/Script/Engine.PlayerController|SetbShowMouseCursor _returnvalue true))
    (:then_2
      (Class|CreatureOasisBlueprintLibrary|StopLoadingScreen)
      (bind _returnvalue_3 (UserInterface|CreateWidget "/Game/CreatureOasis/Core/UI/WBP_FadeInFadeOut.WBP_FadeInFadeOut_C"))
      (UserInterface|Viewport|AddtoViewport _returnvalue_3 0))
    (:then_3
      (Audio|PlaySound2D "/Game/CreatureOasis/Core/Music/chao_l_m.chao_l_m" 1.0 1.0 0.0 0 0))))

(fn ConstructionScript)

(fn GetActiveTrackGenerator
  (return (Variables|Default|GetActiveTrackGenerator)))

(fn SpawnCreatures
  (bind (_outspawnpoints _returnvalue) (Class|TrackGeneratorActor|GetSpawnPoints (Variables|Default|GetActiveTrackGenerator)))
  (if _returnvalue
    (for _index (range 0 2)
      (bind _returnvalue_2 (AI|SpawnAIFromClass "/Game/CreatureOasis/Core/Characters/Chao/Blueprints/BP_ChaoCharacter.BP_ChaoCharacter_C" "/Game/CreatureOasis/Core/Characters/Chao/AI/BehaviorTrees/Racing/BT_CreatureRaceBehavior.BT_CreatureRaceBehavior" (+ (Transformation|GetWorldLocation (.OutItem (Utilities|Array|Random _outspawnpoints))) "0,0,75.000000") (Transformation|GetWorldRotation (.OutItem (Utilities|Array|Random _outspawnpoints))) true 0))
      (Utilities|FlowControl|Sequence
        (:then_0
          (Utilities|Array|Add (Variables|Default|GetSpawnedCreatures) _returnvalue_2))
        (:then_1
          (GameplayEffects|ApplyGameplayEffectToSelf :self (Ability|GetAbilitySystemComponent _returnvalue_2) :GameplayEffectClass "/Game/CreatureOasis/Core/Characters/Chao/GameplayEffects/Racing/GE_WaitForStartSignal_BP.GE_WaitForStartSignal_BP_C"))))))

(fn DestroySpawnedCreatures
  (for _array_element (Variables|Default|GetSpawnedCreatures)
    (Actor|DestroyActor _array_element))
  (Utilities|Array|Clear (Variables|Default|GetSpawnedCreatures)))

(fn GetActiveSplineOfTrackGeneratorActor
  (return (Class|TrackGeneratorActor|GetSplineComponent (CallFunction|GetActiveTrackGenerator))))

(fn GetActiveTrackGeneratorActor
  (return (CallFunction|GetActiveTrackGenerator)))