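; Climbable wall trigger volume that automatically carries a CreatureCharacter upward while it overlaps the box.
; On begin overlap, a dot product check confirms the creature faces against the box's forward vector, then stores it, plays the looping climb montage and disables its movement mode.
; Tick raises the stored creature at constant speed without sweeping.
; End overlap restores walking, stops the montage, plays a climb-out sound and clears the reference.
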(event OnComponentBeginOverlap(CollisionComponent)
  (params (OverlappedComponent :type Primitive%20Component%20Object%20Reference) (OtherActor :type Actor%20Object%20Reference) (OtherComp :type Primitive%20Component%20Object%20Reference) (OtherBodyIndex :type Integer) (bFromSweep :type Boolean) (SweepResult :type Hit%20Result%20Structure%20%28by%20ref%29))
  (bind _ascreature_character (Utilities|Casting|CastToCreatureCharacter OtherActor))
  (if (< (Math|Vector|DotProduct (Transformation|GetActorForwardVector) (Transformation|GetActorForwardVector _ascreature_character)) 0.0)
    (Variables|Default|SetAs%20Creature%20Character _ascreature_character)
    (Animation|PlayAnimMontage _ascreature_character "/Game/CreatureOasis/Art/Characters/Chao/Animations/Montages/AM_ClimbingActions.AM_ClimbingActions" 1.0 "Climb_loop_00")
    (Pawn|Components|CharacterMovement|SetMovementMode (Variables|/Script/Engine.Character|GetCharacterMovement _ascreature_character) "MOVE_None" 0)))

(event OnComponentEndOverlap(CollisionComponent)
  (params (OverlappedComponent :type Primitive%20Component%20Object%20Reference) (OtherActor :type Actor%20Object%20Reference) (OtherComp :type Primitive%20Component%20Object%20Reference) (OtherBodyIndex :type Integer))
  (if (== OtherActor (Variables|Default|GetAs%20Creature%20Character))
    (Pawn|Components|CharacterMovement|SetMovementMode (Variables|/Script/Engine.Character|GetCharacterMovement (Variables|Default|GetAs%20Creature%20Character)) "MOVE_Walking" 0)
    (Animation|StopAnimMontage (Variables|Default|GetAs%20Creature%20Character) "/Game/CreatureOasis/Art/Characters/Chao/Animations/Montages/AM_ClimbingActions.AM_ClimbingActions")
    (Audio|PlaySoundatLocation "/Game/CreatureOasis/Art/Characters/Chao/Sounds/SC_ClimbOut.SC_ClimbOut" (Transformation|GetActorLocation (Variables|Default|GetAs%20Creature%20Character)) "0, 0, 0" 1.0 1.0 0.0 0 0 0 0)
    (Variables|Default|SetAs%20Creature%20Character 0)))

(event EventTick
  (params (DeltaSeconds :type Float%20%28single-precision%29))
  (bind _as_creature_character (Variables|Default|GetAs%20Creature%20Character)
    (:then
      (Transformation|AddActorWorldOffset _as_creature_character (* "0,0,60.000000" DeltaSeconds)))
    (:else)))

(fn ConstructionScript)