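; Chaos Drive interactable that can be held, granting a gameplay effect to a creature when that creature lets go of it.
; On BeginPlay, its subtype tag selects a DT_ChaosDrives row that supplies the effect and the dynamic material's color.
; While simulating physics, a short downward trace each tick triggers upward force for a hover.
; A creature's release applies the effect, then launches the drive along that creature's forward vector.
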(event EventBeginPlay
  (CallFunction|InitialiseChaosDriveTable)
  (CallFunction|UpdateMaterial))

(event EventTick
  (params (DeltaSeconds :type Float%20%28single-precision%29))
  (bind _returnvalue (Transformation|GetActorLocation))
  (bind _staticmesh (Variables|Default|GetStaticMesh))
  (if (Physics|IsSimulatingPhysics _staticmesh "None")
    (bind _returnvalue_2 (Collision|LineTraceByChannel _returnvalue (+ _returnvalue (* (Transformation|GetActorUpVector) -7e+01)) "TraceTypeQuery1" false 0 "None"))
    (if _returnvalue_2
      (Physics|AddForce _staticmesh "0, 0,275000.000000" "None" false))))

(event EventEndBeingHold
  (bind _characterholdingus (Variables|Default|GetCharacterHoldingUs))
  (Utilities|FlowControl|Sequence
    (:then_0
      (bind _returnvalue (Class|HoldableInterface|GetTypeOfActor(Message) _characterholdingus))
      (if (== _returnvalue "(TagName=\"Type.Creature\")")
        (Variables|Default|SetReleasedByCreature (== _returnvalue "(TagName=\"Type.Creature\")"))
        (Variables|Default|SetImpulseToApply (* (Transformation|GetActorForwardVector _characterholdingus) 4e+02))
        (GameplayEffects|ApplyGameplayEffectToSelf :self (Ability|GetAbilitySystemComponent (Variables|Default|GetCharacterHoldingUs)) :GameplayEffectClass (.OnUsedGameplayEffect (Utilities|Struct|BreakChaosDriveTableRow (Variables|Default|GetChaosDriveRow))))))
    (:then_1
      (|CallParentFunction))
    (:then_2
      (if (Variables|Default|GetReleasedByCreature)
        (Physics|AddImpulse (Variables|Default|GetStaticMesh) (Variables|Default|GetImpulseToApply) "None" true)))))

(fn ConstructionScript
  (|CallParentFunction))

(fn InitialiseChaosDriveTable
  (bind (_outname _returnvalue) (Class|CreatureOasisBlueprintLibrary|GetNameOfTopMostChildTag (Variables|Default|GetSubTypeTag)))
  (if _returnvalue
    (bind _returnvalue_2 (Utilities|GetDataTableRow "/Game/CreatureOasis/Core/Interactables/ChaosDrives/DT_ChaosDrives.DT_ChaosDrives" _outname)
      (:then
        (Variables|Default|SetChaosDriveRow _returnvalue_2)))))

(fn ApplyEffect)

(fn UpdateMaterial
  (bind _returnvalue (Rendering|Material|CreateDynamicMaterialInstance (Variables|Default|GetStaticMesh) 0 "/Game/CreatureOasis/Art/Meshes/M_ChaosDrive.M_ChaosDrive" "None" :!class /Script/Engine.PrimitiveComponent))
  (Rendering|Material|SetVectorParameterValue _returnvalue "ChaosDriveColor" (.ColorOverride (Utilities|Struct|BreakChaosDriveTableRow (Variables|Default|GetChaosDriveRow))) :!class /Script/Engine.MaterialInstanceDynamic)
  (Rendering|Material|SetMaterial (Variables|Default|GetStaticMesh) 0 _returnvalue))