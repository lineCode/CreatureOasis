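; Base Blueprint for fruit interactables, configured by a gameplay tag that it exposes through a getter.
; The last dot-separated segment of the tag serves as the row name for looking up and caching fruit data from a data table.
; The construction script runs this lookup and, when a row is found, applies its static mesh, or a fallback mesh if none is set.
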(event EventBeginPlay)

(event Collision|EventActorBeginOverlap
  (params (OtherActor :type Actor%20Object%20Reference)))

(event EventTick
  (params (DeltaSeconds :type Float%20%28single-precision%29)))

(fn ConstructionScript
  (CallFunction|RegenerateFruit))

(fn InitialiseFruitTableRow
  (bind _gameplaytag (Variables|Default|GetGameplayTag))
  (bind _returnvalue (GameplayTags|GetTagName _gameplaytag))
  (bind _returnvalue_2 (Utilities|String|ToString(Name) _returnvalue))
  (bind _returnvalue_3 (Utilities|String|ParseIntoArray _returnvalue_2 "."))
  (bind _returnvalue_4 (Utilities|GetDataTableRow (Variables|Default|GetDataTable) (Utilities|String|StringToName (Utilities|Array|Get(acopy) _returnvalue_3 (Utilities|Array|LastIndex _returnvalue_3))))
    (:then
      (Variables|Default|SetFruitTableRow _returnvalue_4)
      (return true))
    (:RowNotFound
      (return false))))

(fn RegenerateFruit
  (bind _fruittablerow (Variables|Default|GetFruitTableRow))
  (bind _success (CallFunction|InitialiseFruitTableRow))
  (if _success
    (Components|StaticMesh|SetStaticMesh (Variables|Default|GetStaticMesh) (select (!= (.staticmesh _fruittablerow) 0) (.staticmesh _fruittablerow) (Variables|Default|GetFallbackMesh)))))

(fn GetGameplayTag
  (return (Variables|Default|GetGameplayTag)))