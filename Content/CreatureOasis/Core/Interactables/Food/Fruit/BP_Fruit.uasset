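; Holdable fruit actor that is eaten bite by bite, applying gameplay effects to the eater.
; Its data table row is picked by the last segment of the fruit type tag, falling back to "Regular", and sets the mesh at construction.
; Each bite shrinks the mesh and applies a per-bite effect; the final bite applies the depleted effect and destroys the actor.
; Being held disables physics and collision until release.
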(event EventStartBeingHold
  (params (CharacterInstigator :type GAS%20Character%20Object%20Reference))
  (Variables|Default|SetCharacterCurrentlyHoldingUs CharacterInstigator)
  (Physics|SetSimulatePhysics (Variables|Default|GetStaticMesh) false)
  (Collision|SetCollisionEnabled (Variables|Default|GetStaticMesh) "NoCollision"))

(event EventEndBeingHold
  (Variables|Default|SetCharacterCurrentlyHoldingUs 0)
  (Physics|SetSimulatePhysics (Variables|Default|GetStaticMesh) true)
  (Collision|SetCollisionEnabled (Variables|Default|GetStaticMesh) "QueryAndPhysics"))

(event EventBeginPlay
  (|CallParentFunction)
  (CallFunction|InitialiseFruitTableRow))

(fn ConstructionScript
  (CallFunction|RegenerateFruit))

(fn InitialiseFruitTableRow
  (bind _fruittypetag (Variables|Default|GetFruitTypeTag))
  (bind _datatable (Variables|Default|GetDataTable))
  (bind _returnvalue (GameplayTags|GetTagName _fruittypetag))
  (bind _returnvalue_2 (Utilities|String|ToString(Name) _returnvalue))
  (bind _returnvalue_3 (Utilities|String|ParseIntoArray _returnvalue_2 "."))
  (bind _returnvalue_4 (Utilities|GetDataTableRow _datatable (Utilities|String|StringToName (Utilities|Array|Get(acopy) _returnvalue_3 (Utilities|Array|LastIndex _returnvalue_3))))
    (:then
      (Variables|Default|SetFruitTableRow _returnvalue_4))
    (:RowNotFound
      (bind _returnvalue_5 (Utilities|GetDataTableRow _datatable "Regular")
        (:then
          (Variables|Default|SetFruitTableRow _returnvalue_5)))))
  (return))

(fn RegenerateFruit
  (bind _fruittablerow (Variables|Default|GetFruitTableRow))
  (CallFunction|InitialiseFruitTableRow)
  (Components|StaticMesh|SetStaticMesh (Variables|Default|GetStaticMesh) (select (Utilities|IsValid (.staticmesh _fruittablerow)) (.staticmesh _fruittablerow) (Variables|Default|GetFallbackMesh))))

(fn ProcessBite
  (params (Instigator :type Actor%20Object%20Reference))
  (bind _returnvalue (Ability|GetAbilitySystemComponent Instigator))
  (bind _bitestaken (Variables|Default|GetBitesTaken))
  (bind _fruittablerow (Variables|Default|GetFruitTableRow))
  (bind (_gameplaytag _staticmesh _meshscaleoverride _maxportions _perbitegameplayeffect _ondepletedgameplayeffect) (Utilities|Struct|BreakFruitTableRow _fruittablerow))
  (bind _result (Math|Integer|IncrementInt _bitestaken)
    (:%20%20
      (if (< _result _maxportions)
        (Transformation|SetWorldScale3D (Variables|Default|GetStaticMesh) (* (/ _meshscaleoverride _maxportions) (- _maxportions _bitestaken)))
        (GameplayEffects|ApplyGameplayEffectToSelf :self _returnvalue :GameplayEffectClass _perbitegameplayeffect)
        (return false)
        (else
          (GameplayEffects|ApplyGameplayEffectToSelf :self _returnvalue :GameplayEffectClass _ondepletedgameplayeffect)
          (Actor|DestroyActor)
          (return true))))))

(fn GetCharacterCurrentlyHoldingUs
  (return (Variables|Default|GetCharacterCurrentlyHoldingUs)))

(fn GetTypeOfActor
  (return (Variables|Default|GetFruitTypeTag)))

(fn IsBeingHeld
  (return (Utilities|IsValid (Variables|Default|GetCharacterCurrentlyHoldingUs))))