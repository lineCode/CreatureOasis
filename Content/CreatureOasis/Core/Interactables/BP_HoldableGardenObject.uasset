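; Garden object that a character can pick up, carry and throw, exposing its holder, held state and sub-type tag.
; While held, its static mesh has physics simulation and collision disabled; on release both are restored.
; If the holder is moving or was jumping at release, a mass-independent impulse throws the mesh forward and upward relative to that character.
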(event EventStartBeingHold
  (params (CharacterInstigator :type GAS%20Character%20Object%20Reference))
  (bind _staticmesh (Variables|Default|GetStaticMesh))
  (Variables|Default|SetCharacterHoldingUs CharacterInstigator)
  (Physics|SetSimulatePhysics _staticmesh false)
  (Collision|SetCollisionEnabled _staticmesh "NoCollision"))

(event EventEndBeingHold
  (bind _staticmesh (Variables|Default|GetStaticMesh))
  (Utilities|FlowControl|Sequence
    (:then_0
      (Physics|SetSimulatePhysics _staticmesh true)
      (Collision|SetCollisionEnabled _staticmesh "QueryAndPhysics"))
    (:then_1
      (CallFunction|AddImpulsewhenBeingThrown))
    (:then_2
      (Variables|Default|SetCharacterHoldingUs 0))))

(fn ConstructionScript)

(fn AddImpulsewhenBeingThrown
  (bind _characterholdingus (Variables|Default|GetCharacterHoldingUs))
  (bind _characterholdingus_2 (Variables|Default|GetCharacterHoldingUs))
  (if (or (not (Math|Vector|VectorIsNearlyZero (Transformation|GetVelocity _characterholdingus_2))) (Variables|/Script/Engine.Character|GetbWasJumping _characterholdingus_2))
    (Physics|AddImpulse (Variables|Default|GetStaticMesh) (* (+ (Transformation|GetActorForwardVector _characterholdingus) (* (Transformation|GetActorUpVector _characterholdingus) 1.1)) 5e+02) "None" true)))

(fn GetCharacterCurrentlyHoldingUs
  (return (Variables|Default|GetCharacterHoldingUs)))

(fn GetTypeOfActor
  (return (Variables|Default|GetSubTypeTag)))

(fn IsBeingHeld
  (return (Utilities|IsValid (Variables|Default|GetCharacterHoldingUs))))