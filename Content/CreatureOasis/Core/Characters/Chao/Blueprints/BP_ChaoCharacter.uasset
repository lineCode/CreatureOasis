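; Blueprint for the Chao creature character, handling its initial colours and face.
; Construction and BeginPlay both set primary and secondary colours through AppearanceComponent via GenerateRandomColor, whose random-colour node is left unconnected.
; Construction also swaps the middle mouth texture on its dynamic material and sets happy eyes through ExpressionComponent using a gameplay tag.
; StartHold and EndHold are stubs that return false.
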(event EventBeginPlay
  (bind _returnvalue (Utilities|GenerateRandomColor))
  (bind _appearancecomponent (Variables|Default|GetAppearanceComponent))
  (Class|CreatureAppearanceComponent|SetPrimaryColor _appearancecomponent _returnvalue)
  (Class|CreatureAppearanceComponent|SetSecondaryColor _appearancecomponent _returnvalue))

(fn ConstructionScript
  (bind _returnvalue (Utilities|GenerateRandomColor))
  (bind _mesh (Variables|Character|GetMesh))
  (bind _appearancecomponent (Variables|Default|GetAppearanceComponent))
  (Class|CreatureAppearanceComponent|SetPrimaryColor _appearancecomponent _returnvalue)
  (Class|CreatureAppearanceComponent|SetSecondaryColor _appearancecomponent _returnvalue)
  (bind _asmaterial_instance_dynamic (Utilities|Casting|CastToMaterialInstanceDynamic (Rendering|Material|GetMaterial _mesh (Rendering|Material|GetMaterialIndex _mesh "M_mouth_middle"))))
  (Rendering|Material|SetTextureParameterValue _asmaterial_instance_dynamic "MiddleMouthTexture" "/Game/CreatureOasis/Art/Characters/Chao/Textures/Mouth/al_mouth04.al_mouth04")
  (Class|CreatureExpressionComponent|SetEyeTag (Variables|Default|GetExpressionComponent) "(TagName=\"FaceExpression.Chao.Eyes.Happy\")"))

(fn StartHold
  (params (InstigatorActor :type Actor%20Object%20Reference))
  (return false))

(fn EndHold
  (return false))