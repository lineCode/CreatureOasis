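; Gameplay ability for a Chao creature being held, active until an EndBeingHeld gameplay event arrives.
; It plays the held montage at zero rate as a static pose and clears eye and mouth expressions.
; If an ability-system attribute exceeds a threshold, a delay leads to an upset emote-ball effect and uneasy face tags.
; Ending stops the montage, cancels pending tasks and removes the emote effect by its stored handle.
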(event Ability|EventActivateAbility
  (Utilities|FlowControl|Sequence
    (:then_0
      (bind _asynctaskproxy (|PlayMontageandWaitProxy "None" "/Game/CreatureOasis/Art/Characters/Chao/Animations/Montages/AM_BeingHeldActions.AM_BeingHeldActions" 0.0 "Regular_00" true 1.0 0.0)
        (:then
          (Variables|Default|SetAsync%20Task _asynctaskproxy)
          (bind _returnvalue (Class|CreatureComponentGetterInterface|GetCreatureExpressionComponent(Message) (Ability|GetAvatarActorfromActorInfo)))
          (bind _output_get (Variables|Default|SetExpressionComponentRef _returnvalue))
          (Class|CreatureExpressionComponent|ClearEyeandMouthTag _output_get)
          (Ability|Tasks|WaitGameplayEvent "(TagName=\"Event.Interactable.EndBeingHeld\")" 0 true
            (:EventReceived
              (Ability|EndAbility))))))
    (:then_1
      (if (> (.ReturnValue (Ability|Attribute|GetFloatAttributefromAbilitySystemComponent (Ability|GetAbilitySystemComponentfromActorInfo) "(AttributeName=\"Tiredness\",Attribute=/Script/CreatureOasis.ChaoCoreAttributeSet:Tiredness,AttributeOwner=Class'\"/Script/CreatureOasis.ChaoCoreAttributeSet\"')")) 5.0)
        (bind _asynctaskproxy_2 (GameplayTasks|TaskWaitDelay 0 1.0)
          (:then
            (Variables|Default|SetAsync%20Task_0 _asynctaskproxy_2))
          (:OnFinish
            (bind _returnvalue_2 (Ability|ApplyGameplayEffectToOwner "/Game/CreatureOasis/Core/Characters/Chao/GameplayEffects/EmoteBall/GE_EmoteBall_Reaction_Upset_BP.GE_EmoteBall_Reaction_Upset_BP_C"))
            (Variables|Default|SetEmoteBallEffectToRemove _returnvalue_2)
            (Class|CreatureExpressionComponent|SetEyeTag (Variables|Default|GetExpressionComponentRef) "(TagName=\"FaceExpression.Creature.Eyes.ClosedHalf\")")
            (Class|CreatureExpressionComponent|SetMouthTag (Variables|Default|GetExpressionComponentRef) "(TagName=\"FaceExpression.Creature.Mouth.Squiggly\")")))))))

(event Ability|EventOnEndAbility
  (params (bWasCancelled :type Boolean))
  (Animation|Montage|MontageStop -1.0)
  (Utilities|FlowControl|Sequence
    (:then_0
      (bind _async_task (Variables|Default|GetAsync%20Task)
        (:then
          (GameplayTasks|EndTask _async_task))
        (:else)))
    (:then_1
      (bind _async_task_0 (Variables|Default|GetAsync%20Task_0)
        (:then
          (GameplayTasks|EndTask _async_task_0))
        (:else)))
    (:then_2
      (Ability|RemoveGameplayEffectFromOwnerWithHandle (Variables|Default|GetEmoteBallEffectToRemove)))))