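; Chao gameplay ability that plays montages on request through gameplay events, with emote ball effects driven by the animation.
; A PlayMontage event's payload object supplies the montage, a random start section and a time range; after a random delay, it clears effects, finishes the requester's latent task and stops the montage.
; EmoteBall events during playback apply mapped gameplay effects, storing handles for removal.
; An EndMontage event only stops the montage.
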(event Ability|EventActivateAbility
  (Ability|Tasks|WaitGameplayEvent "(TagName=\"Event.Chao.EndMontage\")" 0
    (:then
      (bind _payload (Ability|Tasks|WaitGameplayEvent "(TagName=\"Event.Chao.PlayMontage\")" 0)
        (:EventReceived
          (bind _asplay_montage_gameplay_event_object (Utilities|Casting|CastToPlayMontageGameplayEventObject (.OptionalObject (Utilities|Struct|BreakGameplayEventData _payload))))
          (bind _output_get (Variables|Default|SetAs%20Play%20Montage%20Gameplay%20Event%20Object _asplay_montage_gameplay_event_object))
          (if (not (Utilities|Array|IsEmpty (Variables|/Script/CreatureOasis.PlayMontageGameplayEventObject|GetSectionNames _output_get)))
            (bind _eventtag (|PlayMontageandWaitforEvent "None" (Variables|/Script/CreatureOasis.PlayMontageGameplayEventObject|GetMontageToPlay _output_get) "(GameplayTags=((TagName=\"Event.EmoteBall\")))" 1.0 (.OutItem (Utilities|Array|Random (Variables|/Script/CreatureOasis.PlayMontageGameplayEventObject|GetSectionNames _output_get))) true 1.0)
              (:then
                (Ability|Tasks|WaitDelay (Math|Random|RandomFloatinRange (Variables|/Script/CreatureOasis.PlayMontageGameplayEventObject|GetMinTime _output_get) (Variables|/Script/CreatureOasis.PlayMontageGameplayEventObject|GetMaxTime _output_get))
                  (:OnFinish
                    (CallFunction|ClearEmoteBallEffects)
                    (Class|PlayMontageGameplayEventObject|FinishLatentTaskUsingTaskNode _output_get)
                    (Animation|Montage|MontageStop -1.0))))
              (:EventReceived
                (bind _returnvalue (Ability|ApplyGameplayEffectToOwner (.Value (Utilities|Map|Find (Variables|Default|GetGameplay%20Effect%20Class) _eventtag))))
                (Utilities|Array|Add (Variables|Default|GetEmoteBallEffectHandles) _returnvalue)))))))
    (:EventReceived
      (Animation|Montage|MontageStop -1.0))))

(fn ClearEmoteBallEffects
  (for _array_element (Variables|Default|GetEmoteBallEffectHandles)
    (Ability|RemoveGameplayEffectFromOwnerWithHandle _array_element)))