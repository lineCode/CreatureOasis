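; Gameplay ability for Chao characters that reacts when the player comes within holdable-detection range while the Chao's hands are free.
; On activation it caches the Chao's HoldableAnchor and binds to its detection sphere's overlap, cancelling if the avatar is not a Chao.
; Overlaps with a player-tagged actor's detection-channel primitive play the "GiveMe" reaction montage; no actual holding happens here.
; It is meant to stay active, printing an error if it ends.
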(event Custom|OnDetectionSphereComponentBeginOverlap
  (params (OverlappedComponent :type Primitive%20Component%20Object%20Reference) (OtherActor :type Actor%20Object%20Reference) (OtherComp :type Primitive%20Component%20Object%20Reference) (OtherBodyIndex :type Integer) (bFromSweep :type Boolean) (SweepResult :type Hit%20Result%20Structure%20%28by%20ref%29))
  (if (not (Class|HoldableAnchorComponent|IsHoldingActor (Variables|Default|GetHoldableAnchorRef)))
    (bind _result (CallFunction|IsOverlappingPlayerDetectionPrimitive OtherActor OtherComp))
    (if _result
      (|PlayMontageandWaitforEvent :MontageToPlay "/Game/CreatureOasis/Art/Characters/Chao/Animations/Montages/AM_Reactions.AM_Reactions" :StartSection "GiveMe_Start"))))

(event Ability|EventActivateAbility
  (bind _returnvalue (Ability|GetAvatarActorfromActorInfo))
  (Utilities|IsValid _returnvalue
    (:Is%20Valid
      (bind _asbp_chao_character (Utilities|Casting|CastToBP_ChaoCharacter _returnvalue)
        (:then
          (Variables|Default|SetHoldableAnchorRef (Variables|/Game/CreatureOasis/Core/Characters/Chao/Blueprints/BP_ChaoCharacter.BP_ChaoCharacter_C|GetHoldableAnchor _asbp_chao_character))
          (Collision|BindEventtoOnComponentBeginOverlap (Variables|/Game/CreatureOasis/Core/Characters/Chao/Blueprints/BP_ChaoCharacter.BP_ChaoCharacter_C|GetHoldableDetectionSphere _asbp_chao_character) (EventDispatchers|CreateEvent :!event Custom|OnDetectionSphereComponentBeginOverlap)))
        (:CastFailed
          (Ability|CancelAbility :!label _label))))
    (:Is%20Not%20Valid
      (goto _label))))

(event Ability|EventOnEndAbility
  (params (bWasCancelled :type Boolean))
  (Development|PrintString (Utilities|String|Append (Utilities|GetDisplayName self) " " "Shouldn't have ended") true true "(R=1.000000,G=0.000000,B=0.000000,A=1.000000)" 6.0))

(fn IsOverlappingPlayerDetectionPrimitive
  (params (OtherActor :type Actor%20Object%20Reference) (OtherComponent :type Primitive%20Component%20Object%20Reference))
  (bind _returnvalue (Ability|GetAbilitySystemComponent OtherActor))
  (return (Math|Boolean|ANDBoolean (Utilities|IsValid _returnvalue) (GameplayTags|HasAllMatchingGameplayTags _returnvalue (GameplayTags|MakeLiteralGameplayTagContainer "(GameplayTags=((TagName=\"Type.Player\"),(TagName=\"Ability.HoldActor\")))")) (Utilities|Enum|Equal(Enum) (Collision|GetCollisionObjectType OtherComponent) "ECC_GameTraceChannel3"))))