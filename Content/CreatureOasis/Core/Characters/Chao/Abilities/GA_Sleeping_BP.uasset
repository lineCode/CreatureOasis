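; Gameplay ability that runs a Chao's sleep cycle and its idle animations.
; Attribute-threshold tasks step through falling-asleep, sleeping and waking effects, then end the ability.
; In parallel, a self-restarting random-delay loop jumps between sections of the active montage, choosing variations by whether the Stand animation tag is present.
; Ending the ability stops tracked delay tasks, and cancellation also applies a force-wake effect.
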(event Custom|PlayAction
  (bind _shiftingsectionnames (Variables|Default|GetShiftingSectionNames))
  (if (GameplayTags|HasMatchingGameplayTag (Ability|GetAbilitySystemComponentfromActorInfo) "(TagName=\"State.Chao.Animation.Stand\")")
    (bind _asynctaskproxy (GameplayTasks|TaskWaitDelay 0 (Math|Random|RandomFloatinRange 9.0 3e+01))
      (:then
        (Utilities|Array|Add (Variables|Default|GetAsyncTasks) _asynctaskproxy))
      (:OnFinish
        (Utilities|FlowControl|Sequence
          (:then_0
            (switch int (Math|Random|RandomIntegerinRange 0 2)
              (:0
                (CallFunction|PlayAnimSection (.OutItem (Utilities|Array|Random (Variables|Default|GetPoriSectionNames))))
                (Utilities|Array|Clear (Variables|Default|GetAsyncTasks) :!label _label)
                (CallFunction|PlayAction))
              (:1
                (bind _output_get (Variables|Default|SetTempShiftingAnimIndex (Math|Random|RandomIntegerinRange 0 1)))
                (CallFunction|PlayAnimSection (Utilities|Array|Get(acopy) _shiftingsectionnames _output_get))
                (bind _asynctaskproxy_2 (GameplayTasks|TaskWaitDelay 0 (Math|Random|RandomFloatinRange 8.0 22.0))
                  (:then
                    (Utilities|Array|Add (Variables|Default|GetAsyncTasks) _asynctaskproxy_2))
                  (:OnFinish
                    (CallFunction|PlayAnimSection (Utilities|Array|Get(acopy) _shiftingsectionnames (+ (Variables|Default|GetTempShiftingAnimIndex) 2)))
                    (goto _label))))
              (:2
                (CallFunction|PlayAnimSection "Sleep_belly_00")
                (bind _asynctaskproxy_3 (GameplayTasks|TaskWaitDelay 0 (Math|Random|RandomFloatinRange 8.0 3e+01))
                  (:then
                    (Utilities|Array|Add (Variables|Default|GetAsyncTasks) _asynctaskproxy_3))
                  (:OnFinish
                    (CallFunction|PlayAnimSection "Sleep_belly_00_Reverse")
                    (bind _asynctaskproxy_4 (GameplayTasks|TaskWaitDelay 0 4.0)
                      (:then
                        (Utilities|Array|Add (Variables|Default|GetAsyncTasks) _asynctaskproxy_4))
                      (:OnFinish
                        (goto _label)))))))))))
    (else
      (bind _asynctaskproxy_5 (GameplayTasks|TaskWaitDelay 0 (Math|Random|RandomFloatinRange 7.0 3e+01))
        (:then
          (Utilities|Array|Add (Variables|Default|GetAsyncTasks) _asynctaskproxy_5))
        (:OnFinish
          (CallFunction|PlayAnimSection "Sleep_sit_01")
          (CallFunction|PlayAction))))))

(event Custom|SetSleepEffects
  (bind _returnvalue (Ability|GetAbilitySystemComponentfromActorInfo))
  (bind _returnvalue_2 (GameplayEffects|ApplyGameplayEffectToSelf :self _returnvalue :GameplayEffectClass "/Game/CreatureOasis/Core/Characters/Chao/GameplayEffects/Sleep/GE_Sleep_FallingAsleep_BP.GE_Sleep_FallingAsleep_BP_C"))
  (Variables|Default|SetSleepEffect _returnvalue_2)
  (bind (_asynctaskproxy _bmatchescomparison) (Ability|Tasks|WaitForAttributeChangeThreshold "(AttributeName=\"Tiredness\",Attribute=/Script/CreatureOasis.ChaoCoreAttributeSet:Tiredness,AttributeOwner=Class'\"/Script/CreatureOasis.ChaoCoreAttributeSet\"')" "GreaterThanOrEqualTo" 1e+02 true 0)
    (:then
      (bind (_asynctaskproxy_2 _bmatchescomparison_2) (Ability|Tasks|WaitForAttributeChangeThreshold "(AttributeName=\"Sleepiness\",Attribute=/Script/CreatureOasis.ChaoCoreAttributeSet:Sleepiness,AttributeOwner=Class'\"/Script/CreatureOasis.ChaoCoreAttributeSet\"')" "LessThanOrEqualTo" 0.0 true 0)
        (:OnChange
          (if _bmatchescomparison_2
            (GameplayTasks|EndTask _asynctaskproxy_2)
            (bind _returnvalue_3 (GameplayEffects|ApplyGameplayEffectToSelf :self _returnvalue :GameplayEffectClass "/Game/CreatureOasis/Core/Characters/Chao/GameplayEffects/Sleep/GE_Sleep_Waking_BP.GE_Sleep_Waking_BP_C"))
            (Variables|Default|SetApplyWakingUpEffect _returnvalue_3)
            (bind (_asynctaskproxy_3 _bmatchescomparison_3) (Ability|Tasks|WaitForAttributeChangeThreshold "(AttributeName=\"Tiredness\",Attribute=/Script/CreatureOasis.ChaoCoreAttributeSet:Tiredness,AttributeOwner=Class'\"/Script/CreatureOasis.ChaoCoreAttributeSet\"')" "LessThanOrEqualTo" 0.0 true 0)
              (:OnChange
                (if _bmatchescomparison_3
                  (GameplayTasks|EndTask _asynctaskproxy_3)
                  (Ability|EndAbility)
                  (GameplayEffects|RemoveActiveGameplayEffect _returnvalue (Variables|Default|GetApplyWakingUpEffect) -1))))))))
    (:OnChange
      (if _bmatchescomparison
        (GameplayTasks|EndTask _asynctaskproxy)
        (GameplayEffects|RemoveActiveGameplayEffect _returnvalue (Variables|Default|GetSleepEffect) -1)
        (bind _returnvalue_4 (GameplayEffects|ApplyGameplayEffectToSelf :self _returnvalue :GameplayEffectClass "/Game/CreatureOasis/Core/Characters/Chao/GameplayEffects/Sleep/GE_Sleep_Sleeping_BP.GE_Sleep_Sleeping_BP_C"))
        (Variables|Default|SetApplySleepingEffect _returnvalue_4)))))

(event Ability|EventActivateAbility
  (Utilities|FlowControl|Sequence
    (:then_0
      (CallFunction|SetSleepEffects))
    (:then_1
      (CallFunction|PlayAction))))

(event Ability|EventOnEndAbility
  (params (bWasCancelled :type Boolean))
  (bind _asynctasks (Variables|Default|GetAsyncTasks))
  (Utilities|FlowControl|Sequence
    (:then_0
      (for _array_element _asynctasks
        (GameplayTasks|EndTask _array_element))
      (Utilities|Array|Clear _asynctasks))
    (:then_1
      (if bWasCancelled
        (Ability|ApplyGameplayEffectToOwner (Variables|Default|GetForceWakeEffect))))))

(fn PlayAnimSection
  (params (SectionName :type Name))
  (bind _returnvalue (Class|GameplayAbility|GetOwningComponentfromActorInfo))
  (bind _returnvalue_2 (Components|SkeletalMesh|GetAnimInstance _returnvalue))
  (Ability|Animation|MontageJumptoSection _returnvalue_2 SectionName (Animation|Montage|GetCurrentActiveMontage _returnvalue_2)))