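; GA_PickUpInteractable_BP is the Gameplay Ability a Chao uses to pick up an interactable.
; It sends a start-interact message to the AI controller's current focus actor, passing the Chao character.
; After a short delay it activates the holding-interactable ability by gameplay tag, then ends itself.
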(event Ability|EventActivateAbility
  (bind _returnvalue (Ability|GetAvatarActorfromActorInfo))
  (bind _asbp_chao_character (Utilities|Casting|CastToBP_ChaoCharacter _returnvalue))
  (Class|BPIInteractableActorInterface|StartInteract(Message) (Class|AIController|GetFocusActor (AI|GetAIController _returnvalue)) _asbp_chao_character)
  (Ability|Tasks|WaitDelay 0.5
    (:OnFinish
      (Abilities|TryActivateAbilitiesbyTag (Ability|GetAbilitySystemComponentfromActorInfo) (GameplayTags|MakeGameplayTagContainerfromArray (Utilities|Array|MakeArray (Variables|Default|GetHoldingInteractableGameplayTag))) true)
      (Ability|EndAbility))))

(event Ability|EventOnEndAbility
  (params (bWasCancelled :type Boolean)))