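; Gameplay ability for a Chao's regular thinking behavior, playing an idle think montage for a few seconds.
; It starts the montage at a random section from its list, cancelling if the list is empty, and ends itself after a random delay.
; A montage event applies the thinking emote-ball gameplay effect, which is removed by handle when the ability ends.
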(event Ability|EventActivateAbility
  (bind _sectiontochoosefrom (Variables|Default|GetSectionToChooseFrom))
  (if (Utilities|Array|IsEmpty _sectiontochoosefrom)
    (Ability|CancelAbility)
    (else
      (|PlayMontageandWaitforEvent "None" "/Game/CreatureOasis/Art/Characters/Chao/Animations/Montages/AM_IdleThink.AM_IdleThink" "(GameplayTags=((TagName=\"Event.EmoteBall.Thinking\")))" 1.0 (.OutItem (Utilities|Array|Random _sectiontochoosefrom)) true 1.0
        (:then
          (Ability|Tasks|WaitDelay (Math|Random|RandomFloatinRange 2.75 4.0)
            (:OnFinish
              (Ability|EndAbility))))
        (:EventReceived
          (bind _returnvalue (Ability|ApplyGameplayEffectToOwner "/Game/CreatureOasis/Core/Characters/Chao/GameplayEffects/EmoteBall/GE_EmoteBall_Reaction_Thinking_BP.GE_EmoteBall_Reaction_Thinking_BP_C"))
          (Variables|Default|SetEmoteBallEffectHandle _returnvalue))))))

(event Ability|EventOnEndAbility
  (params (bWasCancelled :type Boolean))
  (Ability|RemoveGameplayEffectFromOwnerWithHandle (Variables|Default|GetEmoteBallEffectHandle)))