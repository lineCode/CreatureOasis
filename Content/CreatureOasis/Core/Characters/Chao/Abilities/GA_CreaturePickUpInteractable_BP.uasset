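; Gameplay ability that lets a Chao creature pick up the interactable its AI controller is focused on.
; On activation it plays the start-eat-fruit montage on the Chao and waits out its duration.
; It then sends a start-being-held message to the focus actor, activates abilities tagged for holding an interactable, and ends.
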(event Ability|EventActivateAbility
  (bind _returnvalue (Ability|GetAvatarActorfromActorInfo))
  (bind _asbp_chao_character (Utilities|Casting|CastToBP_ChaoCharacter _returnvalue))
  (bind _returnvalue_2 (Animation|PlayAnimMontage _asbp_chao_character "/Game/CreatureOasis/Art/Characters/Chao/Animations/Montages/AM_StartEatFruit.AM_StartEatFruit" 1.0 "None"))
  (Ability|Tasks|WaitDelay _returnvalue_2
    (:OnFinish
      (Class|HoldableInterface|StartBeingHold(Message) (Class|AIController|GetFocusActor (AI|GetAIController _returnvalue)) _asbp_chao_character)
      (Abilities|TryActivateAbilitiesbyTag (Ability|GetAbilitySystemComponentfromActorInfo) (GameplayTags|MakeGameplayTagContainerfromArray (Utilities|Array|MakeArray (Variables|Default|GetHoldingInteractableGameplayTag))) true)
      (Ability|EndAbility))))

(event Ability|EventOnEndAbility
  (params (bWasCancelled :type Boolean)))