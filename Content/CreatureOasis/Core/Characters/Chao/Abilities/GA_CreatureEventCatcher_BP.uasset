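; Gameplay Ability for Chao creatures that catches gameplay events and turns them into reactions, currently to having a held item taken away.
; On activation it waits for Event.HoldCancel events and tracks the async task so it can end it with the ability.
; When the event's target tags include State.Holdable.TakenAway and a checked attribute exceeds a threshold, it applies the food-taken-away reaction effect to itself.
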(event Custom|ListenForHoldCancelEvent
  (bind _returnvalue (Ability|GetAbilitySystemComponentfromActorInfo))
  (bind (_asynctaskproxy _payload) (Ability|Tasks|WaitGameplayEvent "(TagName=\"Event.HoldCancel\")" 0)
    (:then
      (Utilities|Array|Add (Variables|Default|GetAsyncTasks) _asynctaskproxy))
    (:EventReceived
      (if (GameplayTags|HasTag (.TargetTags (Utilities|Struct|BreakGameplayEventData _payload)) "(TagName=\"State.Holdable.TakenAway\")" true)
        (if (> (.ReturnValue (Ability|Attribute|GetFloatAttributefromAbilitySystemComponent _returnvalue "(AttributeName=\"Hunger\",Attribute=/Script/CreatureOasis.ChaoCoreAttributeSet:Hunger,AttributeOwner=Class'\"/Script/CreatureOasis.ChaoCoreAttributeSet\"')")) 5e+01)
          (GameplayEffects|ApplyGameplayEffectToSelf :self _returnvalue :GameplayEffectClass "/Game/CreatureOasis/Core/Characters/Chao/GameplayEffects/GE_FoodTakenAwayReaction_BP.GE_FoodTakenAwayReaction_BP_C"))))))

(event Ability|EventActivateAbility
  (CallFunction|ListenforHoldCancelEvent))

(event Ability|EventOnEndAbility
  (params (bWasCancelled :type Boolean))
  (for _array_element (Variables|Default|GetAsyncTasks)
    (Utilities|IsValid _array_element
      (:Is%20Valid
        (GameplayTasks|EndTask _array_element)))))